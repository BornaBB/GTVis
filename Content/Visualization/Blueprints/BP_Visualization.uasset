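; BP_Visualization is an actor holding visualization meshes for a main flow and the intake, rotor and exhaust of a big and a small compartment.
; The construction script sets each mesh's visibility from its own boolean.
; Tick caches the cast game state, then polls its interaction mode and hides all seven meshes during Mechanical Exploration.
; Nothing in this graph shows them again when the mode changes.
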(event `self.ReceiveTick`
  (params (DeltaSeconds :type "Float (single-precision)"))
  (bind _gamestate (`self.GameState`)
    (:`then`
      (bind _returnvalue (`self.GetInteractionMode` _gamestate))
      (switch `|SwitchEnum` _returnvalue
        (:`MechanicalExploration`
          (`SceneComponent.SetVisibility` (`self.SM_Visualization_Main_Flow`) false false)
          (`SceneComponent.SetVisibility` (`self.SM_Visualization_Big_Rotor`) false false)
          (`SceneComponent.SetVisibility` (`self.SM_Visualization_Mini_Rotor`) false false)
          (`SceneComponent.SetVisibility` (`self.SM_Visualization_Big_Intake`) false false)
          (`SceneComponent.SetVisibility` (`self.SM_Visualization_Big_Exhaust`) false false)
          (`SceneComponent.SetVisibility` (`self.SM_Visualization_Mini_Intake`) false false)
          (`SceneComponent.SetVisibility` (`self.SM_Visualization_Mini_Exhaust`) false false))))
    (:`else`
      (bind _asse_game_state (cast `` (`GameplayStatics.GetGameState`)))
      (set `self.GameState` _asse_game_state))))

(fn `UserConstructionScript`
  (`SceneComponent.SetVisibility` (`self.SM_Visualization_Main_Flow`) (`self.Main Flow`) false)
  (`SceneComponent.SetVisibility` (`self.SM_Visualization_Big_Intake`) (`self.Big Compartment - Intake`) false)
  (`SceneComponent.SetVisibility` (`self.SM_Visualization_Big_Rotor`) (`self.Big Compartment - Rotor`) false)
  (`SceneComponent.SetVisibility` (`self.SM_Visualization_Big_Exhaust`) (`self.Big Compartment - Exhaust`) false)
  (`SceneComponent.SetVisibility` (`self.SM_Visualization_Mini_Intake`) (`self.Small Compartment - Intake`) false)
  (`SceneComponent.SetVisibility` (`self.SM_Visualization_Mini_Rotor`) (`self.Small Compartment - Rotor`) false)
  (`SceneComponent.SetVisibility` (`self.SM_Visualization_Mini_Exhaust`) (`self.Small Compartment - Exhaust`) false))